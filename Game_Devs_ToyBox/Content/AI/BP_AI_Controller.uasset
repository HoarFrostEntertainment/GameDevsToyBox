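; AI controller that runs a behavior tree on BeginPlay and feeds AI Perception updates into its Blackboard.
; Hearing stimuli re-set bHearNew and store the sound location as InvestLoc for investigation.
; A sight update sets the actor as Target while any actor remains seen.
; When none remain, it clears Target and reuses bHearNew and InvestLoc to flag that actor's current location.
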(event `self.ReceiveBeginPlay`
  (`self.RunBehaviorTree` (`self.BTAsset`)))

(event `self.AIPerception.OnTargetPerceptionUpdated`
  (params (Actor :type "Actor Object Reference") (Stimulus :type "AIStimulus Structure"))
  (bind _blackboard (`self.Blackboard`))
  (bind _returnvalue (`AIPerceptionSystem.GetSenseClassForStimulus` Stimulus))
  (if (== _returnvalue "/Script/AIModule.AISense_Hearing")
    (`BlackboardComponent.ClearValue` _blackboard "bHearNew")
    (`BlackboardComponent.SetValueAsBool` _blackboard "bHearNew" true)
    (`BlackboardComponent.SetValueAsVector` _blackboard "InvestLoc" (`.StimulusLocation` (break `AIStimulus` Stimulus)))
    (elif (== _returnvalue "/Script/AIModule.AISense_Sight")
      (if (== (`KismetArrayLibrary.Array_Length` (`AIPerceptionComponent.GetPerceivedActors` (`self.AIPerception`) "/Script/AIModule.AISense_Sight")) 0)
        (`BlackboardComponent.ClearValue` _blackboard "Target")
        (`BlackboardComponent.SetValueAsBool` _blackboard "bHearNew" true)
        (`BlackboardComponent.SetValueAsVector` _blackboard "InvestLoc" (`self.K2_GetActorLocation` Actor))
        (else
          (`BlackboardComponent.SetValueAsObject` _blackboard "Target" Actor))))))

(fn `UserConstructionScript`)