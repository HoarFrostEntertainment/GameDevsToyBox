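; TargetBP is a shooting-range target prop that reacts to being hit and then resets itself.
; A skeletal mesh hit from anything other than the player pawn shows a hit marker widget for the local player and plays the shot-down animation.
; A Down flag ignores further hits until the reset animation plays after a short delay and clears it.
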(event `self.SkeletalMesh.OnComponentHit`
  (params (HitComponent :type "PrimitiveComponent Object Reference") (OtherActor :type "Actor Object Reference") (OtherComp :type "PrimitiveComponent Object Reference") (NormalImpulse :type "Vector Structure") (Hit :type "HitResult Structure (by ref)"))
  (if (== (`GameplayStatics.GetPlayerPawn` 0) OtherActor)
    _
    (elif (not (`self.down`))
      (bind _returnvalue (`|CreateWidget` "/Game/Game_Devs_ToyBox/FPShooter_ToyBox/HUD_UI/HitMarker/HitMarker.HitMarker_C" (`GameplayStatics.GetPlayerController` 0)))
      (`UserWidget.AddToViewport` _returnvalue 0)
      (`SkeletalMeshComponent.PlayAnimation` (`self.SkeletalMesh`) "/Game/Game_Devs_ToyBox/FPShooter_ToyBox/Props/BulletTargets/Animation/Human_Target_Shot.Human_Target_Shot" false)
      (set `self.down` true)
      (`KismetSystemLibrary.Delay` 5.0)
      (`SkeletalMeshComponent.PlayAnimation` (`self.SkeletalMesh`) "/Game/Game_Devs_ToyBox/FPShooter_ToyBox/Props/BulletTargets/Animation/Human_Target_Reset.Human_Target_Reset" false)
      (set `self.down` false))))

(fn `UserConstructionScript`)